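; A coin pickup actor that the first-person character collects by overlapping its Box.
; On overlap it increments the character's Coincollected count, prints the new total and destroys itself.
; A Rotation function yaws the root, but the looping BeginPlay timer targets the misspelled name "rotaion", which matches no function shown here.
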(event `self.ReceiveBeginPlay`
  (`KismetSystemLibrary.K2_SetTimer` null "rotaion" 0.005 true))

(event `self.Box.OnComponentBeginOverlap`
  (params (OverlappedComponent :type "PrimitiveComponent Object Reference") (OtherActor :type "Actor Object Reference") (OtherComp :type "PrimitiveComponent Object Reference") (OtherBodyIndex :type Integer) (bFromSweep :type Boolean) (SweepResult :type "HitResult Structure (by ref)"))
  (bind _asbp_first_person_character (cast `/Game/FirstPerson/Blueprints/BP_FirstPersonCharacter` OtherActor))
  (bind _output_get (set `/Game/FirstPerson/Blueprints/BP_FirstPersonCharacter.coincollected` (+ (`/Game/FirstPerson/Blueprints/BP_FirstPersonCharacter.coincollected` _asbp_first_person_character) 1) _asbp_first_person_character))
  (`KismetSystemLibrary.PrintString` (`KismetStringLibrary.Conv_IntToString` _output_get) true true (struct :`R` 1.0 :`G` 0.031677 :`A` 1.0))
  (`self.K2_DestroyActor`))

(fn `rotation`
  (`SceneComponent.K2_AddLocalRotation` (`self.DefaultSceneRoot`) (`KismetMathLibrary.MakeRotator` 0.0 0.0 10.0) false false))

(fn `UserConstructionScript`)