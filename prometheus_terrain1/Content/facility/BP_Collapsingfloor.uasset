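; BP_Collapsingfloor is a floor tile that gives a warning and then collapses after the first-person player steps on it.
; A box overlap by BP_FirstPersonCharacter starts a timer, apparently leading to a warning that plays a sound and changes the point light's intensity.
; The warning sets a second timer, apparently for the drop, which enables physics on the tile and gives the actor a short lifespan.
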(event `self.Box.OnComponentBeginOverlap`
  (params (OverlappedComponent :type "PrimitiveComponent Object Reference") (OtherActor :type "Actor Object Reference") (OtherComp :type "PrimitiveComponent Object Reference") (OtherBodyIndex :type Integer) (bFromSweep :type Boolean) (SweepResult :type "HitResult Structure (by ref)"))
  (cast `/Game/FirstPerson/Blueprints/BP_FirstPersonCharacter` OtherActor)
  (`KismetSystemLibrary.K2_SetTimerDelegate` (`|CreateDelegate` :!event `warning`) (`self.WarningDuration`)))

(event `warning`
  (`GameplayStatics.PlaySound2D` "/Game/facility/UI_SFX_Free_Pack/Cues/Cancel/cancel_1_Cue.cancel_1_Cue" 1.0 1.0 0.0 null null)
  (`LightComponent.SetIntensity` (`self.PointLight`) (`self.ActiveIntensity`))
  (`KismetSystemLibrary.K2_SetTimerDelegate` (`|CreateDelegate` :!event `DropTile`) (`self.AfterWarningDuration`)))

(event `DropTile`
  (`PrimitiveComponent.SetSimulatePhysics` (`self.tile`) true)
  (`self.SetLifeSpan` 1.0))

(fn `UserConstructionScript`)